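; Pawn possessed for the in-game menu, placed at the first-person camera, hosting main menu, inventory and journal sections under a ribbon widget.
; Input events switch sections by fading out the active widget, then opening the next or returning to the game.
; The inventory spawns 3D item actors, with timer-driven interpolation for cycling and close-up inspection.
; Tick sphere-traces toward the selected item to smoothly adjust depth-of-field focus.
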(event `self.ReceiveTick`
  (params (DeltaSeconds :type "Float (single-precision)"))
  ;[0 0.7682 1] Adjust depth of field
  (`self.AdjustFocalDistance`))

(event `self.ReceivePossessed`
  (params (NewController :type "Controller Object Reference"))
  (bind _returnvalue (`GameplayStatics.GetPlayerController` 0))
  (bind _gamecontroller (`self.GameController`))
  (bind _gamepawn (`/Game/StoryAdvTemplate/Blueprints/BP_GameController.GamePawn` _gamecontroller))
  ;[0 0.7682 1] Initialize menu when pawn is possessed
  (bind _asbp_first_person_character (cast `/Game/StoryAdvTemplate/Blueprints/BP_FirstPersonCharacter` _gamepawn))
  (bind (_cameraposition _camerarotation) (`/Game/StoryAdvTemplate/Blueprints/BP_FirstPersonCharacter.GetCameraPosition` _asbp_first_person_character))
  (`self.K2_SetActorLocationAndRotation` (`/Game/StoryAdvTemplate/Blueprints/BP_GameController.MenuPawn` _gamecontroller) _cameraposition _camerarotation false true)
  (`Controller.SetControlRotation` (`GameplayStatics.GetPlayerController` 0) (`self.GetControlRotation` _gamepawn))
  (if (== NewController _returnvalue)
    (`self.HideOtherWidgets`)
    (bind _returnvalue_2 (`|CreateWidget` "/Game/StoryAdvTemplate/UserInterface/Menu/UI_MenuRibbon.UI_MenuRibbon_C" null self (`self.GamepadInput`) (`self.SearchForKey`)))
    (bind _output_get (set `self.Ribbon` _returnvalue_2))
    (`UserWidget.AddToViewport` _output_get 0)
    (`self.DisableInput` (`self.GameController`) _returnvalue)
    (`/Game/StoryAdvTemplate/Blueprints/BP_FirstPersonCharacter.GetCameraPosition` _asbp_first_person_character)
    (switch `/Game/StoryAdvTemplate/Blueprints/Core/GameMenu/EMenuSection` (`self.ActiveMenu`)
      (:`NewEnumerator0`
        (`self.OpenMenu`))
      (:`NewEnumerator1`
        (`self.CreateInventory`))
      (:`NewEnumerator2`
        (`self.OpenJournal`)))))

(event `self.ReceiveUnpossessed`
  (params (OldController :type "Controller Object Reference"))
  ;[0 0.7682 1] Remove menu when pawn is unpossessed
  (`self.UnhideOtherWidgets`)
  (bind _ribbon (`self.Ribbon`)
    (:`then`
      (`Widget.RemoveFromParent` _ribbon)
      (set `/Game/StoryAdvTemplate/Blueprints/BP_GameController.SearchForKey` false (`self.GameController`)))
    (:`else`)))

(event `OpenMenu`
  (bind _returnvalue (`GameplayStatics.GetPlayerController` 0))
  (bind _gamepadinput (`self.GamepadInput`))
  ;[0 0.7682 1] Open Game Menu
  (`KismetSystemLibrary.Delay` 0.1)
  (bind _returnvalue_2 (`|CreateWidget` "/Game/StoryAdvTemplate/UserInterface/Menu/UI_GameMenu.UI_GameMenu_C" null (`self.GamepadInput`) self))
  (set `self.GameMenu` _returnvalue_2)
  (if (not (`Widget.IsInViewport` (`self.GameMenu`)))
    (`UserWidget.AddToViewport` (`self.GameMenu`) 0))
  (if (not _gamepadinput)
    (`WidgetBlueprintLibrary.SetInputMode_GameAndUIEx` _returnvalue null))
  (set `PlayerController.bShowMouseCursor` (not _gamepadinput) _returnvalue)
  (`KismetSystemLibrary.Delay` 0.1)
  (bind _output_get (set `self.ActiveMenu` "NewEnumerator0"))
  (`/Game/StoryAdvTemplate/UserInterface/Menu/UI_MenuRibbon.ChangeSelection` (`self.Ribbon`) _output_get)
  (`KismetSystemLibrary.Delay` 0.5)
  (`self.EnableInput` (`GameplayStatics.GetPlayerController` 0))
  (set `self.ActionInputEnabled` true))

(event `CloseGameMenu`
  (params (BackToGame :type Boolean) (OpenNext :type "/Game/StoryAdvTemplate/Blueprints/Core/GameMenu/EMenuSection Enum" :default "NewEnumerator0"))
  (bind _returnvalue (`GameplayStatics.GetPlayerController` 0))
  ;[0 0.7682 1] Close Game Menu
  (set `self.BackToGame` BackToGame)
  (set `self.NextSection` OpenNext)
  (bind _gamemenu (`self.GameMenu`)
    (:`then`
      (bind _fadein (`/Game/StoryAdvTemplate/UserInterface/Menu/UI_GameMenu.FadeIn` _gamemenu))
      (`UserWidget.PlayAnimation` _gamemenu _fadein 0.0 1 "Reverse" 2.0 false)
      (`|ExecutionSequence`
        (:`then_0`
          (if (`self.BackToGame`) :!label _label
            (bind _ribbon (`self.Ribbon`)
              (:`then`
                (`UserWidget.PlayAnimation` _ribbon (`/Game/StoryAdvTemplate/UserInterface/Menu/UI_MenuRibbon.FadeIn` _ribbon) 0.0 1 "Reverse" 2.0 false))
              (:`else`))))
        (:`then_1`
          (`KismetSystemLibrary.Delay` (`WidgetAnimation.GetEndTime` _fadein))
          (bind _gamemenu_2 (`self.GameMenu`)
            (:`then`
              (`Widget.RemoveFromParent` _gamemenu_2))
            (:`else`
              _))
          (set `PlayerController.bShowMouseCursor` false _returnvalue)
          (`WidgetBlueprintLibrary.SetInputMode_GameOnly` _returnvalue)
          (if (`self.BackToGame`)
            (`Widget.RemoveFromParent` (`self.Ribbon`))
            (`/Game/StoryAdvTemplate/Blueprints/BP_GameController.CloseMenu` (`self.GameController`))
            (else
              (switch `/Game/StoryAdvTemplate/Blueprints/Core/GameMenu/EMenuSection` (`self.NextSection`)
                (:`NewEnumerator1`
                  (`self.CreateInventory`))
                (:`NewEnumerator2`
                  (`self.OpenJournal`))))))))
    (:`else`
      (goto _label))))

(event `CloseInventory`
  (params (BackToGame :type Boolean) (OpenNext :type "/Game/StoryAdvTemplate/Blueprints/Core/GameMenu/EMenuSection Enum" :default "NewEnumerator0"))
  (bind _returnvalue (`GameplayStatics.GetPlayerController` 0))
  ;[0 0.7682 1] Inventory
  ;;[1 1 1] Close Inventory
  (set `self.BackToGame` BackToGame)
  (set `self.NextSection` OpenNext)
  (bind _inventoryhud (`self.InventoryHUD`)
    (:`then`
      (bind _fadein (`/Game/StoryAdvTemplate/UserInterface/Menu/UI_FullscreenInventory.FadeIn` _inventoryhud))
      (`UserWidget.PlayAnimation` _inventoryhud _fadein 0.0 1 "Reverse" 2.0 false)
      (`|ExecutionSequence`
        (:`then_0`
          (if (`self.BackToGame`) :!label _label_2
            (bind _ribbon (`self.Ribbon`)
              (:`then`
                (`UserWidget.PlayAnimation` _ribbon (`/Game/StoryAdvTemplate/UserInterface/Menu/UI_MenuRibbon.FadeIn` _ribbon) 0.0 1 "Reverse" 2.0 false))
              (:`else`))))
        (:`then_1`
          (`KismetSystemLibrary.Delay` (`WidgetAnimation.GetEndTime` _fadein))
          (bind _inventoryhud_2 (`self.InventoryHUD`)
            (:`then`
              (`Widget.RemoveFromParent` _inventoryhud_2))
            (:`else`
              _))
          (set `PlayerController.bShowMouseCursor` false _returnvalue)
          (`WidgetBlueprintLibrary.SetInputMode_GameOnly` _returnvalue)
          (bind _selecteditem (`self.SelectedItem`)
            (:`then`
              (`self.K2_DestroyActor` _selecteditem))
            (:`else`
              _))
          (if (`self.BackToGame`)
            (`Widget.RemoveFromParent` (`self.Ribbon`))
            (`/Game/StoryAdvTemplate/Blueprints/BP_GameController.CloseMenu` (`self.GameController`))
            (else
              (switch `/Game/StoryAdvTemplate/Blueprints/Core/GameMenu/EMenuSection` (`self.NextSection`)
                (:`NewEnumerator0`
                  (`self.OpenMenu`))
                (:`NewEnumerator2`
                  (`self.OpenJournal`))))))))
    (:`else`
      (goto _label_2))))

(event `OpenJournal`
  (bind _returnvalue (`GameplayStatics.GetPlayerController` 0))
  (bind _gamepadinput (`self.GamepadInput`))
  ;[0 0.7682 1] Journal
  ;;[1 1 1] Open Journal
  (`KismetSystemLibrary.Delay` 0.1)
  (bind _returnvalue_2 (`|CreateWidget` "/Game/StoryAdvTemplate/UserInterface/Menu/UI_Journal.UI_Journal_C"))
  (bind _output_get (set `self.Journal` _returnvalue_2))
  (`UserWidget.AddToViewport` _output_get 0)
  (if (not _gamepadinput)
    (`WidgetBlueprintLibrary.SetInputMode_GameAndUIEx` _returnvalue null))
  (set `PlayerController.bShowMouseCursor` (not _gamepadinput) _returnvalue)
  (`KismetSystemLibrary.Delay` 0.1)
  (bind _output_get_2 (set `self.ActiveMenu` "NewEnumerator2"))
  (`/Game/StoryAdvTemplate/UserInterface/Menu/UI_MenuRibbon.ChangeSelection` (`self.Ribbon`) _output_get_2)
  (`self.EnableInput` (`GameplayStatics.GetPlayerController` 0))
  (set `self.ActionInputEnabled` true))

(event `CreateInventory`
  ;[0 0.7682 1] Inventory
  ;;[1 1 1] Create widget, spawn items if possible, change menu ribbon selection, enable input
  (bind _returnvalue (`|CreateWidget` "/Game/StoryAdvTemplate/UserInterface/Menu/UI_FullscreenInventory.UI_FullscreenInventory_C"))
  (bind _output_get (set `self.InventoryHUD` _returnvalue))
  (`UserWidget.AddToViewport` _output_get 0)
  (bind _actor (`self.SpawnItemActor` (`self.SelectedItemLocation`) (`self.SelectedItemIndex`)))
  (set `self.SelectedItem` _actor)
  (bind _output_get_2 (set `self.ActiveMenu` "NewEnumerator1"))
  (`/Game/StoryAdvTemplate/UserInterface/Menu/UI_MenuRibbon.ChangeSelection` (`self.Ribbon`) _output_get_2)
  (`KismetSystemLibrary.Delay` 0.5)
  (`self.EnableInput` (`GameplayStatics.GetPlayerController` 0))
  (set `self.ActionInputEnabled` true))

(event `CloseJournal`
  (params (BackToGame :type Boolean) (OpenNext :type "/Game/StoryAdvTemplate/Blueprints/Core/GameMenu/EMenuSection Enum" :default "NewEnumerator0"))
  (bind _returnvalue (`GameplayStatics.GetPlayerController` 0))
  ;[0 0.7682 1] Journal
  ;;[1 1 1] Close Journal
  (set `self.BackToGame` BackToGame)
  (set `self.NextSection` OpenNext)
  (bind _journal (`self.Journal`)
    (:`then`
      (bind _fadein (`/Game/StoryAdvTemplate/UserInterface/Menu/UI_Journal.FadeIn` _journal))
      (`UserWidget.PlayAnimation` _journal _fadein 0.0 1 "Reverse" 2.0 false)
      (`|ExecutionSequence`
        (:`then_0`
          (if (`self.BackToGame`) :!label _label_3
            (bind _ribbon (`self.Ribbon`)
              (:`then`
                (`UserWidget.PlayAnimation` _ribbon (`/Game/StoryAdvTemplate/UserInterface/Menu/UI_MenuRibbon.FadeIn` _ribbon) 0.0 1 "Reverse" 2.0 false))
              (:`else`))))
        (:`then_1`
          (`KismetSystemLibrary.Delay` (`WidgetAnimation.GetEndTime` _fadein))
          (bind _journal_2 (`self.Journal`)
            (:`then`
              (`Widget.RemoveFromParent` _journal_2))
            (:`else`
              _))
          (set `PlayerController.bShowMouseCursor` false _returnvalue)
          (`WidgetBlueprintLibrary.SetInputMode_GameOnly` _returnvalue)
          (if (`self.BackToGame`)
            (`Widget.RemoveFromParent` (`self.Ribbon`))
            (`/Game/StoryAdvTemplate/Blueprints/BP_GameController.CloseMenu` (`self.GameController`))
            (else
              (switch `/Game/StoryAdvTemplate/Blueprints/Core/GameMenu/EMenuSection` (`self.NextSection`)
                (:`NewEnumerator0`
                  (`self.OpenMenu`))
                (:`NewEnumerator1`
                  (`self.CreateInventory`))))))))
    (:`else`
      (goto _label_3))))

(event `ReloadInventory`
  (bind _selecteditemindex (`self.SelectedItemIndex`))
  ;[0 0.7682 1] Inventory
  ;;[1 1 1] Remove item and create inventory new
  (`|ExecutionSequence`
    (:`then_0`
      (bind _selecteditem (`self.SelectedItem`)
        (:`then`
          (`self.K2_DestroyActor` _selecteditem))
        (:`else`)))
    (:`then_1`
      (set `self.SelectedItemIndex` (select `bool` (`KismetArrayLibrary.Array_IsValidIndex` (`/Game/StoryAdvTemplate/Blueprints/BP_GameController.Inventory` (`self.GameController`)) _selecteditemindex) :`true` _selecteditemindex))
      (bind _actor (`self.SpawnItemActor` (`self.SelectedItemLocation`) (`self.SelectedItemIndex`)))
      (set `self.SelectedItem` _actor)
      (`/Game/StoryAdvTemplate/UserInterface/Menu/UI_MenuRibbon.SwitchSelectedItem` (`self.Ribbon`))
      (set `self.ActionInputEnabled` true))))

(event `InputAction|GameMenu` :paused true
  (params (Key :type "Key Structure"))
  ;[0 0.7682 1] Handle quick selection input
  ;;[1 1 1] Game Menu Key
  (:`Pressed`
    (`self.GameMenuButton`)))

(event `GameMenuButton`
  ;[0 0.7682 1] Handle quick selection input
  ;;[1 1 1] Game Menu Key
  (if (and (`self.ActionInputEnabled`) (not (`self.InspectMode`)))
    (set `self.ActionInputEnabled` false)
    (switch `/Game/StoryAdvTemplate/Blueprints/Core/GameMenu/EMenuSection` (`self.ActiveMenu`)
      (:`NewEnumerator0`
        (`self.CloseGameMenu` true))
      (:`NewEnumerator1`
        (`self.CloseInventory` true))
      (:`NewEnumerator2`
        (`self.CloseJournal` true)))))

(event `InputAction|PreviousMenuSection` :paused true
  (params (Key :type "Key Structure"))
  ;[0 0.7682 1] Toggle Menu Section
  ;;[1 1 1] Switch to previous section
  (:`Pressed`
    (if (and (`self.ActionInputEnabled`) (not (`self.InspectMode`)) (not (`self.SearchForKey`)))
      (switch `/Game/StoryAdvTemplate/Blueprints/Core/GameMenu/EMenuSection` (`self.ActiveMenu`)
        (:`NewEnumerator0`
          (`self.CloseGameMenu` false "NewEnumerator2"))
        (:`NewEnumerator1`
          (`self.CloseInventory` false))
        (:`NewEnumerator2`
          (`self.CloseJournal` false "NewEnumerator1")))
      (set `self.ActionInputEnabled` false))))

(event `InputAction|Inventory` :paused true
  (params (Key :type "Key Structure"))
  ;[0 0.7682 1] Handle quick selection input
  ;;[1 1 1] Inventory Key
  (:`Pressed`
    (`self.InventoryButton`)))

(event `InventoryButton`
  ;[0 0.7682 1] Handle quick selection input
  ;;[1 1 1] Inventory Key
  (if (and (`self.ActionInputEnabled`) (not (`self.InspectMode`)))
    (set `self.ActionInputEnabled` false)
    (switch `/Game/StoryAdvTemplate/Blueprints/Core/GameMenu/EMenuSection` (`self.ActiveMenu`)
      (:`NewEnumerator0`
        (`self.CloseGameMenu` false "NewEnumerator1"))
      (:`NewEnumerator1`
        (`self.CloseInventory` true))
      (:`NewEnumerator2`
        (`self.CloseJournal` false "NewEnumerator1")))))

(event `InputAction|NextMenuSection` :paused true
  (params (Key :type "Key Structure"))
  ;[0 0.7682 1] Toggle Menu Section
  ;;[1 1 1] Switch to next section
  (:`Pressed`
    (if (and (`self.ActionInputEnabled`) (not (`self.InspectMode`)) (not (`self.SearchForKey`)))
      (switch `/Game/StoryAdvTemplate/Blueprints/Core/GameMenu/EMenuSection` (`self.ActiveMenu`)
        (:`NewEnumerator0`
          (`self.CloseGameMenu` false "NewEnumerator1"))
        (:`NewEnumerator1`
          (`self.CloseInventory` false "NewEnumerator2"))
        (:`NewEnumerator2`
          (`self.CloseJournal` false)))
      (set `self.ActionInputEnabled` false))))

(event `InputAction|Journal` :paused true
  (params (Key :type "Key Structure"))
  ;[0 0.7682 1] Handle quick selection input
  ;;[1 1 1] Journal Key
  (:`Pressed`
    (`self.JournalButton`)))

(event `JournalButton`
  ;[0 0.7682 1] Handle quick selection input
  ;;[1 1 1] Journal Key
  (if (and (`self.ActionInputEnabled`) (not (`self.InspectMode`)) (not (`self.SearchForKey`)))
    (set `self.ActionInputEnabled` false)
    (switch `/Game/StoryAdvTemplate/Blueprints/Core/GameMenu/EMenuSection` (`self.ActiveMenu`)
      (:`NewEnumerator0`
        (`self.CloseGameMenu` false "NewEnumerator2"))
      (:`NewEnumerator1`
        (`self.CloseInventory` false "NewEnumerator2"))
      (:`NewEnumerator2`
        (`self.CloseJournal` true)))))

(fn `AdjustFocalDistance`
  (bind _returnvalue (`SceneComponent.K2_GetComponentLocation` (`self.Camera`)))
  (`/Engine/EditorBlueprintResources/StandardMacros.IsValid` (`self.SelectedItem`)
    (:`Is Valid`
      (bind _outhit (`KismetSystemLibrary.SphereTraceSingle` _returnvalue (+ _returnvalue (* (`KismetMathLibrary.GetDirectionUnitVector` _returnvalue (`self.K2_GetActorLocation` (`self.SelectedItem`))) 5000.0)) 2.0 "TraceTypeQuery1"))
      (bind (_bblockinghit _binitialoverlap _time _distance) (`GameplayStatics.BreakHitResult` _outhit))
      (bind _output_get (set `self.FocalDistance` (`KismetMathLibrary.FInterpTo` (`self.FocalDistance`) (select `bool` _bblockinghit :`false` 20.0 :`true` _distance :!type "Float (double-precision)") (`GameplayStatics.GetWorldDeltaSeconds`) 10.0)))
      (setmembers `PostProcessSettings` :`StructRef` (`CameraComponent.PostProcessSettings` (`self.Camera`)) :`DepthOfFieldFocalDistance` _output_get))))

(fn `HideOtherWidgets`
  (bind _foundwidgets (`WidgetBlueprintLibrary.GetAllWidgetsOfClass` "/Script/UMG.UserWidget"))
  (for _array_element _foundwidgets
    (if (and (!= _array_element (`self.InventoryHUD`)) (`Widget.IsVisible` _array_element))
      (`KismetArrayLibrary.Array_AddUnique` (`self.HiddenWidgets`) _array_element)
      (`Widget.SetVisibility` _array_element "Collapsed"))))

(fn `InspectionInterpolation`
  ;[0 0.7682 1] Move selected item close to camera or back to selected item slot
  (if (and (== (`self.K2_GetActorLocation` (`self.SelectedItem`)) (select `bool` (`self.EndInspection`) :`false` (`self.CloseUpLocation`) :`true` (`self.SelectedItemLocation`)) :`ErrorTolerance` 0.25) (== (`self.K2_GetActorRotation` (`self.SelectedItem`)) (`/Game/StoryAdvTemplate/Blueprints/Core/GameMenu/BP_FullscreenInventoryItem.OriginRotation` (`self.SelectedItem`)) :`ErrorTolerance` 0.25))
    ;;[1 1 1] Stop interpolation, check if player is inspecting after interpolation
    (`KismetSystemLibrary.K2_ClearTimer` null "InspectionInterpolation")
    (set `self.EndInspection` (not (`self.EndInspection`)))
    (set `self.ActionInputEnabled` true)
    (if (`self.EndInspection`)
      ;;[1 1 1] Disable object rotation for letters
      (switch `/Game/StoryAdvTemplate/Blueprints/Data/LetterTypes_Enum` (`.Lettertype_75_5C8F2592441A376C5F8B1BA8DF65AA0B` (break `/Game/StoryAdvTemplate/Blueprints/Data/Structures/BP_InventoryItem` (`|GetArrayItem` (`/Game/StoryAdvTemplate/Blueprints/BP_GameController.Inventory` (`self.GameController`)) (`self.SelectedItemIndex`))))
        (:`NewEnumerator3`
          (set `self.CanTurn` true))
        (:`NewEnumerator0`
          (set `self.CanTurn` false :!label _label)
          (`/Game/StoryAdvTemplate/Blueprints/Core/GameMenu/BP_FullscreenInventoryItem.Inspection` (`self.SelectedItem`)))
        (:`NewEnumerator1`
          (goto _label))
        (:`NewEnumerator2`
          (goto _label)))
      (else
        ;;[1 1 1] Object was put back, enable object rotation and allow shuffle input
        (`Widget.SetVisibility` (`self.InventoryHUD`) "Visible")
        (`Widget.SetVisibility` (`self.Ribbon`) "Visible")
        (set `self.CanTurn` true)
        (set `self.ShuffleAllowed` true)
        (set `self.InspectMode` false)))
    (else
      ;;[1 1 1] Interpolate location and rotation
      (`self.K2_SetActorLocationAndRotation` (`self.SelectedItem`) (`KismetMathLibrary.VInterpTo` (`self.K2_GetActorLocation` (`self.SelectedItem`)) (select `bool` (`self.EndInspection`) :`false` (`self.CloseUpLocation`) :`true` (`self.SelectedItemLocation`)) (`GameplayStatics.GetWorldDeltaSeconds`) (`self.InterpolationSpeed`)) (`KismetMathLibrary.RInterpTo` (`self.K2_GetActorRotation` (`self.SelectedItem`)) (`/Game/StoryAdvTemplate/Blueprints/Core/GameMenu/BP_FullscreenInventoryItem.OriginRotation` (`self.SelectedItem`)) (`GameplayStatics.GetWorldDeltaSeconds`) (`self.InterpolationSpeed`)) false false))))

(fn `NextItemAnimation`
  (bind _returnvalue (+ (`self.SelectedItemIndex`) 1))
  ;[0 0.7682 1] Cycle next item
  ;;[1 1 1] Animate item location
  (if (== (`self.K2_GetActorLocation` (`self.SelectedItem`)) (`self.LastItemLocation`) :`ErrorTolerance` 0.25)
    (`KismetSystemLibrary.K2_ClearTimer` null "NextItemAnimation")
    ;;[1 1 1] Set new selected item index
    (set `self.SelectedItemIndex` (select `bool` (`KismetArrayLibrary.Array_IsValidIndex` (`/Game/StoryAdvTemplate/Blueprints/BP_GameController.Inventory` (`self.GameController`)) _returnvalue) :`true` _returnvalue))
    ;;[1 1 1] Remove out of screen item, set new selected item actor
    (`self.K2_DestroyActor` (`self.SelectedItem`))
    (set `self.SelectedItem` (`self.SecondItem`))
    ;;[1 1 1] Reenable input
    (`self.EnableInput` (`GameplayStatics.GetPlayerController` 0))
    (`/Game/StoryAdvTemplate/UserInterface/Menu/UI_MenuRibbon.SwitchSelectedItem` (`self.Ribbon`))
    (set `self.ActionInputEnabled` true)
    (else
      (`self.Item Interpolation` (`self.SelectedItem`) (`self.LastItemLocation`))
      (`self.Item Interpolation` (`self.SecondItem`) (`self.SelectedItemLocation`)))))

(fn `PreviousItemAnimation`
  (bind _returnvalue (- (`self.SelectedItemIndex`) 1))
  (bind _inventory (`/Game/StoryAdvTemplate/Blueprints/BP_GameController.Inventory` (`self.GameController`)))
  ;[0 0.7682 1] Cycle previous item
  ;;[1 1 1] Animate item location
  (if (== (`self.K2_GetActorLocation` (`self.SelectedItem`)) (`self.SecondItemLocation`) :`ErrorTolerance` 0.25)
    (`KismetSystemLibrary.K2_ClearTimer` null "PreviousItemAnimation")
    ;;[1 1 1] Set new selected item index
    (set `self.SelectedItemIndex` (select `bool` (`KismetArrayLibrary.Array_IsValidIndex` _inventory _returnvalue) :`false` (`KismetArrayLibrary.Array_LastIndex` _inventory) :`true` _returnvalue))
    ;;[1 1 1] Remove out of screen item, set new selected item actor
    (`self.K2_DestroyActor` (`self.SelectedItem`))
    (set `self.SelectedItem` (`self.LastItem`))
    ;;[1 1 1] Reenable input
    (`self.EnableInput` (`GameplayStatics.GetPlayerController` 0))
    (`/Game/StoryAdvTemplate/UserInterface/Menu/UI_MenuRibbon.SwitchSelectedItem` (`self.Ribbon`))
    (set `self.ActionInputEnabled` true)
    (else
      (`self.Item Interpolation` (`self.SelectedItem`) (`self.SecondItemLocation`))
      (`self.Item Interpolation` (`self.LastItem`) (`self.SelectedItemLocation`)))))

(fn `SpawnItemActor`
  (params (SpawnLocation :type "Vector Structure") (InventoryArrayIndex :type Integer))
  (returns (Actor :type "/Game/StoryAdvTemplate/Blueprints/Core/GameMenu/BP_FullscreenInventoryItem Object Reference"))
  (locals (Location :type "Vector Structure") (Index :type Integer) (Mesh :type "StaticMesh Object Reference"))
  (bind ((`ObjectMesh_11_356E5C844C749FF1E8AFBEA055E696E2` _objectmesh) (`UseAction_105_CC970B694408EBA385A5278267034095` _useaction) (`Lettertype_75_5C8F2592441A376C5F8B1BA8DF65AA0B` _lettertype) (`ContainsClue_77_EFF04A5344D8DC7D9B377584FC8F156F` _containsclue)) (break `/Game/StoryAdvTemplate/Blueprints/Data/Structures/BP_InventoryItem` (`|GetArrayItem` (`/Game/StoryAdvTemplate/Blueprints/BP_GameController.Inventory` (`self.GameController`)) (`local.Index`))))
  (set `local.Location` SpawnLocation)
  (set `local.Index` InventoryArrayIndex)
  (if (`KismetArrayLibrary.Array_IsValidIndex` (`/Game/StoryAdvTemplate/Blueprints/BP_GameController.Inventory` (`self.GameController`)) (`local.Index`))
    (set `local.Mesh` _objectmesh)
    (switch `/Game/StoryAdvTemplate/Blueprints/Data/LetterTypes_Enum` _lettertype
      (:`NewEnumerator3`
        (if _containsclue
          (bind _returnvalue (`|SpawnActorFromClass` "/Game/StoryAdvTemplate/Blueprints/Core/GameMenu/BP_FullscreenInventoryItem_Clue.BP_FullscreenInventoryItem_Clue_C" (`KismetMathLibrary.Conv_VectorToTransform` (`local.Location`)) "Undefined" "OverrideRootScale" null (`local.Mesh`) (`self.GameController`) (`local.Index`) null))
          (return _returnvalue)
          (else
            (bind _returnvalue_2 (`|SpawnActorFromClass` "/Game/StoryAdvTemplate/Blueprints/Core/GameMenu/BP_FullscreenInventoryItem.BP_FullscreenInventoryItem_C" (`KismetMathLibrary.Conv_VectorToTransform` (`local.Location`)) "Undefined" "OverrideRootScale" null (`local.Mesh`) (`self.GameController`) (`local.Index`) null))
            (return _returnvalue_2))))
      (:`NewEnumerator0`
        _)
      (:`NewEnumerator1`
        _)
      (:`NewEnumerator2`
        _))
    (bind _returnvalue_3 (`|SpawnActorFromClass` "/Game/StoryAdvTemplate/Blueprints/Core/GameMenu/BP_FullscreenInventoryLetter.BP_FullscreenInventoryLetter_C" (`KismetMathLibrary.Conv_VectorToTransform` (`local.Location`)) "Undefined" "OverrideRootScale" null (`local.Mesh`) (`self.GameController`) (`local.Index`) null))
    (return _returnvalue_3)
    (else
      (return null))))

(fn `UnhideOtherWidgets`
  (for _array_element (`self.HiddenWidgets`)
    (`Widget.SetVisibility` _array_element "Visible"))
  (`KismetArrayLibrary.Array_Clear` (`self.HiddenWidgets`))
  (return))

(fn `UserConstructionScript`)